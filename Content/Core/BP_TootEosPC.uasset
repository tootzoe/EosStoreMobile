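; Player controller for the TootEos project that sets up the main UI and provides on-screen logging.
; On BeginPlay it registers a store offer list view model in the global MVVM collection, under a name taken from BP_MainGameInstance.
; It then creates and shows UI_Main, switches input to Game and UI with a visible cursor, and writes a first log line.
; DoTxtLog appends either a success or failure message to that widget's log.
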(event `self.ReceiveBeginPlay`
  (`self.SetupMVVM`)
  (bind _returnvalue (`|CreateWidget` "/Game/UI/UI_Main.UI_Main_C"))
  (bind _output_get (set `self.MainUIWid` _returnvalue))
  (`/Game/UI/UI_Main.ShowMe` _output_get self)
  (`WidgetBlueprintLibrary.SetInputMode_GameAndUIEx` self _returnvalue)
  (set `self.bShowMouseCursor` true)
  (`self.DoTxtLog` true "Start Logging here..........."))

(fn `DoTxtLog`
  (params (IsOk :type Boolean) (TxtOk :type String) (TxtFail :type String))
  (bind _mainuiwid (`self.MainUIWid`)
    (:`then`
      (if IsOk
        (`/Game/UI/UI_Main.AppendLogInfo` _mainuiwid (`local.TxtOk`))
        (else
          (`/Game/UI/UI_Main.AppendLogInfo` _mainuiwid (`local.TxtFail`))))
      (return))
    (:`else`)))

(fn `SetupMVVM`
  (bind _asbp_main_game_instance (cast `/Game/Core/BP_MainGameInstance` (`GameplayStatics.GetGameInstance`)))
  (bind _returnvalue (`|GenericCreateObject` self "/Game/MVVM/VM_StoreOfferItemList.VM_StoreOfferItemList_C"))
  (bind _returnvalue_2 (`MVVMViewModelCollectionObject.AddViewModelInstance` (`MVVMGameSubsystem.GetViewModelCollection` (subsystem `MVVMGameSubsystem`)) (make `MVVMViewModelContext` "/Game/MVVM/VM_StoreOfferItemList.VM_StoreOfferItemList_C" (`/Game/Core/BP_MainGameInstance.VM_StoreOffersCollectinoName` _asbp_main_game_instance)) _returnvalue))
  (`KismetSystemLibrary.PrintString` (`KismetStringLibrary.Concat_StrStr` "create store offer viewmodel...." (`KismetStringLibrary.Conv_BoolToString` _returnvalue_2))))

(fn `UserConstructionScript`)